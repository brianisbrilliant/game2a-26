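; Quest-giver actor that runs a linear, voiced dialogue with the third-person character on overlap.
; It creates a dialogue widget at BeginPlay, shows it on overlap and registers itself as the player's QuestGiver.
; Each NextLine call reads the next DT_Talk row, sets text, plays audio, and aligns and tilts text by speaker.
; Running out of rows or leaving the sphere resets the index, removes the widget and clears the player's reference.
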(event `self.ReceiveBeginPlay`
  ; Create the dialogue widget
  (bind _returnvalue (`|CreateWidget` "/Game/W_DialogueHolder.W_DialogueHolder_C"))
  (set `self.W_Dialogue` _returnvalue))

(event `self.ReceiveActorBeginOverlap`
  (params (OtherActor :type "Actor Object Reference"))
  (bind _asbp_third_person_character (cast `/Game/ThirdPerson/Blueprints/BP_ThirdPersonCharacter` OtherActor))
  (bind _output_get (set `self.player` _asbp_third_person_character))
  (`KismetSystemLibrary.PrintText` (`KismetTextLibrary.Conv_StringToText` (`KismetSystemLibrary.GetDisplayName` _output_get)))
  ; add the widget to the viewport
  (`UserWidget.AddToViewport` (`self.W_Dialogue`) 0)
  (set `/Game/ThirdPerson/Blueprints/BP_ThirdPersonCharacter.QuestGiver` self _output_get)
  (`self.Next Line`))

(event `self.Sphere.OnComponentEndOverlap`
  (params (OverlappedComponent :type "PrimitiveComponent Object Reference") (OtherActor :type "Actor Object Reference") (OtherComp :type "PrimitiveComponent Object Reference") (OtherBodyIndex :type Integer))
  (cast `/Game/ThirdPerson/Blueprints/BP_ThirdPersonCharacter` OtherActor)
  (`self.End of Dialogue` :!label _label))

(event `Next Line`
  (bind _datatablerowindex (`self.DataTableRowIndex`))
  (bind _dialoguetext (`/Game/W_Dialogue.DialogueText` (`/Game/W_DialogueHolder.W_Dialogue` (`self.W_Dialogue`))))
  (`KismetSystemLibrary.PrintText` "requesting next line")
  (bind _outrownames (`DataTableFunctionLibrary.GetDataTableRowNames` (`self.DataTable`)))
  (if (> _datatablerowindex (`KismetArrayLibrary.Array_LastIndex` _outrownames))
    (goto _label)
    (else
      (bind _returnvalue (`|GetDataTableRow` "/Game/DT_Talk.DT_Talk" (`|GetArrayItem` _outrownames _datatablerowindex))
        (:`then`
          (`TextBlock.SetText` _dialoguetext (`KismetTextLibrary.Conv_StringToText` (break `/Game/S_Talk` _returnvalue)))
          (switch `/Game/E_Speakers` (`.Speaker_5_0B17E613D24AE4C359262A84B2F9422F` (break `/Game/S_Talk` _returnvalue))
            (:`NewEnumerator0`
              (set `TextLayoutWidget.Justification` "Left" _dialoguetext)
              (`Widget.SetRenderTransformAngle` _dialoguetext -5.0))
            (:`NewEnumerator1`
              (set `TextLayoutWidget.Justification` "Right" _dialoguetext)
              (`Widget.SetRenderTransformAngle` _dialoguetext 5.0)))
          (`GameplayStatics.PlaySoundAtLocation` (`.Audio_8_6AF67445334BE94D78ACEF80F2801957` (break `/Game/S_Talk` _returnvalue)) (`self.K2_GetActorLocation`) (struct) 1.0 1.0 0.0 null null null null)
          (`/Engine/EditorBlueprintResources/StandardMacros.IncrementInt` (`self.DataTableRowIndex`)))))))

(event `End of Dialogue`
  (set `self.DataTableRowIndex` 0)
  ; remove the widget from the viewport
  (`Widget.RemoveFromParent` (`self.W_Dialogue`))
  (bind _player (`self.player`)
    (:`then`
      (set `/Game/ThirdPerson/Blueprints/BP_ThirdPersonCharacter.QuestGiver` null _player))
    (:`else`)))

(fn `UserConstructionScript`)