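; BP_NPC is a talkable NPC that shows a voiced dialogue widget with optional portraits while the player overlaps its sphere.
; On overlap it registers itself on the player character and shows the first line; leaving hides the widget and resets to the starting line.
; NextLine steps through DT_NPCDialogue rows until a separator marker or the table's end, playing audio and tilting and justifying text by speaker.
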(event `self.ReceiveBeginPlay`
  (bind _w_dialogue (`self.W_Dialogue`))
  (bind _returnvalue (`|CreateWidget` "/Game/Widgets/W_NPDdialogue.W_NPDdialogue_C")) ; Get the widget ready to show
  (set `self.W_Dialogue` _returnvalue)
  (set `self.NextLineIndex` (`self.StartingLineIndex`)) ; Make sure we start talking\non the correct line
  (`|ExecutionSequence`
    (:`then_0`
      (bind _playerport (`self.playerport`) ; Did we set a different \nimage?
        (:`then`
          (`Image.SetBrushFromTexture` (`/Game/Widgets/W_NPDdialogue.Player_Portrait` _w_dialogue) _playerport true))
        (:`else`)))
    (:`then_1`
      (bind _npcport (`self.NPCPort`) ; Did we set a different \nimage?
        (:`then`
          (`Image.SetBrushFromTexture` (`/Game/Widgets/W_NPDdialogue.NPC_Portrait` _w_dialogue) _npcport true))
        (:`else`)))))

(event `self.Sphere.OnComponentBeginOverlap`
  (params (OverlappedComponent :type "PrimitiveComponent Object Reference") (OtherActor :type "Actor Object Reference") (OtherComp :type "PrimitiveComponent Object Reference") (OtherBodyIndex :type Integer) (bFromSweep :type Boolean) (SweepResult :type "HitResult Structure (by ref)"))
  (bind _asbp_third_person_character (cast `/Game/ThirdPerson/Blueprints/BP_ThirdPersonCharacter` OtherActor))
  (bind _output_get (set `self.Player` _asbp_third_person_character))
  (set `/Game/ThirdPerson/Blueprints/BP_ThirdPersonCharacter.NPC` self _output_get) ; Tell the Player that \nthey're talking to US
  (`UserWidget.AddToViewport` (`self.W_Dialogue`) 0)
  (`self.Next Line`))

(event `self.Sphere.OnComponentEndOverlap`
  (params (OverlappedComponent :type "PrimitiveComponent Object Reference") (OtherActor :type "Actor Object Reference") (OtherComp :type "PrimitiveComponent Object Reference") (OtherBodyIndex :type Integer))
  (cast `/Game/ThirdPerson/Blueprints/BP_ThirdPersonCharacter` OtherActor)
  (`self.End Dialogue`))

(event `End Dialogue`
  (set `/Game/ThirdPerson/Blueprints/BP_ThirdPersonCharacter.NPC` null (`self.Player`)) ; Set NPC to null
  (set `self.Player` null) ; Set Player to null
  (`Widget.RemoveFromParent` (`self.W_Dialogue`)) ; Hide the dialogue
  (set `self.NextLineIndex` (`self.StartingLineIndex`)) ; Reset the index
)

(event `Next Line`
  (bind _audio (`self.Audio`))
  (bind _textblock_0 (`/Game/Widgets/W_NPDdialogue.TextBlock_0` (`self.W_Dialogue`)))
  (bind _outrownames (`DataTableFunctionLibrary.GetDataTableRowNames` "/Game/Blueprints/DT_NPCDialogue.DT_NPCDialogue"))
  (if (> (`self.NextLineIndex`) (`KismetArrayLibrary.Array_LastIndex` _outrownames))
    (`self.End Dialogue`)
    (else
      (bind _returnvalue (`|GetDataTableRow` "/Game/Blueprints/DT_NPCDialogue.DT_NPCDialogue" (`|GetArrayItem` _outrownames (`self.NextLineIndex`)))
        (:`then`
          ; Are we at the end of our lines?
          (if (`KismetStringLibrary.EqualEqual_StrStr` (break `/Game/Blueprints/S_NPCDialogue` _returnvalue) "<-------->")
            (`self.End Dialogue`)
            (else
              (`TextBlock.SetText` (`/Game/Widgets/W_NPDdialogue.TextBlock_0` (`self.W_Dialogue`)) (`KismetTextLibrary.Conv_StringToText` (break `/Game/Blueprints/S_NPCDialogue` _returnvalue)))
              (`/Engine/EditorBlueprintResources/StandardMacros.IncrementInt` (`self.NextLineIndex`) ; Increment Int
                (:`  `
                  ; Play the voiced dialogue
                  (`AudioComponent.SetSound` _audio (`.VoicedLine_7_D71E9981F6476ABD2C42DA89C1857F5C` (break `/Game/Blueprints/S_NPCDialogue` _returnvalue)))
                  (`AudioComponent.Play` _audio 0.0)
                  ; Update text in cute ways
                  (`Widget.SetRenderTransformAngle` _textblock_0 (select `/Game/Blueprints/E_Speaker` (`.Speaker_8_14558C99A64E9A80594ED0A8B0D7DB30` (break `/Game/Blueprints/S_NPCDialogue` _returnvalue)) :`NewEnumerator0` (`KismetMathLibrary.RandomFloatInRange` -7.0 -3.0) :`NewEnumerator1` (`KismetMathLibrary.RandomFloatInRange` 3.0 7.0))) ; Rotate the text
                  (set `TextLayoutWidget.Justification` (select `/Game/Blueprints/E_Speaker` (`.Speaker_8_14558C99A64E9A80594ED0A8B0D7DB30` (break `/Game/Blueprints/S_NPCDialogue` _returnvalue)) :`NewEnumerator0` "Left" :`NewEnumerator1` "Right" :!type "ETextJustify Enum") _textblock_0) ; change the justification
                )))))))))

(fn `UserConstructionScript`)