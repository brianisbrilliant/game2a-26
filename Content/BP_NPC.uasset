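; BP_NPC is a talkable NPC that shows dialogue lines in a W_Talk widget, created on BeginPlay.
; When a BP_ThirdPersonCharacter overlaps its sphere, it registers itself as that player's NPC, prints a greeting and adds the widget to the viewport.
; The NextLine event writes the current Dialogue entry to the widget and increments the index, with no bounds check or widget removal.
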(event `self.ReceiveBeginPlay`
  (bind _returnvalue (`|CreateWidget` "/Game/Widgets/W_Talk.W_Talk_C"))
  (set `self.W_Talk` _returnvalue))

(event `self.Sphere.OnComponentBeginOverlap`
  (params (OverlappedComponent :type "PrimitiveComponent Object Reference") (OtherActor :type "Actor Object Reference") (OtherComp :type "PrimitiveComponent Object Reference") (OtherBodyIndex :type Integer) (bFromSweep :type Boolean) (SweepResult :type "HitResult Structure (by ref)"))
  (bind _asbp_third_person_character (cast `/Game/ThirdPerson/Blueprints/BP_ThirdPersonCharacter` OtherActor))
  (bind _output_get (set `self.Player` _asbp_third_person_character))
  (set `/Game/ThirdPerson/Blueprints/BP_ThirdPersonCharacter.NPC` self _output_get) ; Let the player know\nthey're talking to US
  (`KismetSystemLibrary.PrintText` "Hello!")
  (`UserWidget.AddToViewport` (`self.W_Talk`) 0))

(event `Next Line`
  (`TextBlock.SetText` (`/Game/Widgets/W_Talk.TextBlock_0` (`self.W_Talk`)) (`|GetArrayItem` (`self.Dialogue`) (`self.LineIndex`)))
  (`/Engine/EditorBlueprintResources/StandardMacros.IncrementInt` (`self.LineIndex`)))

(fn `UserConstructionScript`)